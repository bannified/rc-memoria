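; BP_PowerUp_MvmtSpeed is a pickup that gives the player a temporary movement speed boost.
; When a BP_PlayerCharacterBase overlaps its Box, it calls MovementSpeedUp with Duration on the character's BPPowerUpComponent.
; It then shows a popup on the character with a hardcoded x2 speed label, adds a WBP_PowerupMask widget to the viewport and destroys itself.
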(event `self.Box.OnComponentBeginOverlap`
  (params (OverlappedComponent :type "PrimitiveComponent Object Reference") (OtherActor :type "Actor Object Reference") (OtherComp :type "PrimitiveComponent Object Reference") (OtherBodyIndex :type Integer) (bFromSweep :type Boolean) (SweepResult :type "HitResult Structure (by ref)"))
  (bind _asbp_player_character_base (cast `/Game/Blueprints/BP_PlayerCharacterBase` OtherActor))
  (`/Game/Blueprints/LootSystem/Powerup/BP_PowerUpComponent.MovementSpeedUp` (`/Game/Blueprints/BP_PlayerCharacterBase.BP_PowerUpComponent` _asbp_player_character_base) (`self.Duration`))
  (`/Game/Widgets/MemoriaWidgetBlueprintFunctionLibrary.ShowEventPopupOnCharacter` (`self.PopupImage`) (`|FormatText` "x{0} movement speed" 2.0) _asbp_player_character_base)
  (bind _returnvalue (`|CreateWidget` "/Game/Widgets/WBP_PowerupMask.WBP_PowerupMask_C"))
  (`UserWidget.AddToViewport` _returnvalue 0)
  (`self.K2_DestroyActor`))

(fn `UserConstructionScript`
  (`parent.UserConstructionScript`))