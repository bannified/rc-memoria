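; Actor component that applies a timed movement speed power-up to its owning BP_PlayerCharacterBase.
; The MovementSpeedUp event multiplies the character's MaxWalkSpeed by SpeedMultiplier, then divides it back once the given duration ends.
; An IsSpeedUp flag prevents stacking, while a retriggerable delay restarts the countdown when the event fires again during an active boost.
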(event `self.ReceiveBeginPlay`)

(event `MovementSpeedUp`
  (params (MovementSpeedUpDuration :type "Float (double-precision)"))
  (bind _asbp_player_character_base (cast `/Game/Blueprints/BP_PlayerCharacterBase` (`self.GetOwner`)))
  (if (not (`self.IsSpeedUp`))
    (bind _charactermovement (`Character.CharacterMovement` _asbp_player_character_base))
    (bind _maxwalkspeed (`CharacterMovementComponent.MaxWalkSpeed` _charactermovement))
    (set `CharacterMovementComponent.MaxWalkSpeed` (* _maxwalkspeed (`self.SpeedMultiplier`)) _charactermovement)
    (set `self.IsSpeedUp` true))
  (`KismetSystemLibrary.RetriggerableDelay` MovementSpeedUpDuration)
  (set `CharacterMovementComponent.MaxWalkSpeed` (/ _maxwalkspeed (`self.SpeedMultiplier`)) _charactermovement)
  (set `self.IsSpeedUp` false))