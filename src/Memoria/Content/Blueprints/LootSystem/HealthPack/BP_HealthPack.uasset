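; BP_HealthPack is a pickup that heals the player character on contact and then destroys itself.
; Its Box overlap event accepts only the first player's pawn, casts it to BP_CharacterBase and passes HealValue to that character's HealthComponent through AlterHealth.
; It then shows an event popup on the character with PopupImage and the heal amount before removing the actor.
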(event `self.ReceiveBeginPlay`
  (`parent.ReceiveBeginPlay`))

(event `self.Box.OnComponentBeginOverlap`
  (params (OverlappedComponent :type "PrimitiveComponent Object Reference") (OtherActor :type "Actor Object Reference") (OtherComp :type "PrimitiveComponent Object Reference") (OtherBodyIndex :type Integer) (bFromSweep :type Boolean) (SweepResult :type "HitResult Structure (by ref)"))
  (bind _returnvalue (`GameplayStatics.GetPlayerPawn` 0))
  (if (== OtherActor _returnvalue)
    (bind _asbp_character_base (cast `/Game/Blueprints/BP_CharacterBase` _returnvalue))
    (`HealthComponent.AlterHealth` (`CharacterBase.HealthComponent` _asbp_character_base) (`self.Heal Value`))
    (if true
      (`/Game/Widgets/MemoriaWidgetBlueprintFunctionLibrary.ShowEventPopupOnCharacter` (`self.PopupImage`) (`|FormatText` "+{0} Health" (`self.Heal Value`)) _asbp_character_base)
      (`self.K2_DestroyActor`))))

(fn `UserConstructionScript`
  (`parent.UserConstructionScript`))