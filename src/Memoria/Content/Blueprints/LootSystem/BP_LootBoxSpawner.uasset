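; BP_LootBoxSpawner is a placeable actor that spawns a BP_LootBox at its location when play begins.
; It passes its item type, healthpack and powerup weights to the box and gives it a back-reference to the spawner.
; Its SpawnDelay event spawns a replacement box after RespawnTime, if the spawner is respawnable.
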(event `self.ReceiveBeginPlay`
  (set `self.SpawnLocation` (`SceneComponent.K2_GetComponentLocation` (`self.DefaultSceneRoot`)))
  (`self.SpawnLootBox`))

(event `SpawnLootBox`
  (bind _returnvalue (`|SpawnActorFromClass` "/Game/Blueprints/LootSystem/BP_LootBox.BP_LootBox_C" (`KismetMathLibrary.Conv_VectorToTransform` (`self.SpawnLocation`)) "Undefined" "OverrideRootScale" null (`self.ItemTypeWeights`) (`self.HealthpackWeights`) (`self.PowerupWeights`) null))
  (set `/Game/Blueprints/LootSystem/BP_LootBox.LootBoxSpawner` self _returnvalue))

(event `SpawnDelay`
  (if (`self.IsRespawnable`)
    (`KismetSystemLibrary.Delay` (`self.RespawnTime`))
    (`self.SpawnLootBox`)))

(fn `UserConstructionScript`)