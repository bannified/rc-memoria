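; BP_ItemSpawn is a loot spawner actor that randomly drops a health pack, a power-up or nothing at its location on BeginPlay.
; ChooseItemType makes a weighted roll through duplicated Select options, favoring no drop, then health packs.
; ChooseItem picks a random row from the matching DataTable and spawns that row's class, passing in its stats, name and the spawner's despawn time.
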(event `self.ReceiveBeginPlay`
  (bind _item_type (`self.Choose Item Type`))
  (`self.Choose Item` _item_type))

(fn `Choose Item`
  (params (`Item Type` :type "/Game/Blueprints/LootSystem/LootTypeEnum Enum" :default "NewEnumerator2"))
  (returns (Item :type "Actor Object Reference"))
  (bind _despawn_time (`self.Despawn Time`))
  (bind _returnvalue (`KismetMathLibrary.Conv_VectorToTransform` (`self.K2_GetActorLocation`)))
  (switch `/Game/Blueprints/LootSystem/LootTypeEnum` `Item Type`
    (:`NewEnumerator2`
      (bind _outrownames (`DataTableFunctionLibrary.GetDataTableRowNames` "/Game/Blueprints/LootSystem/HealthPack/HealthPackDataTable.HealthPackDataTable"))
      (bind _returnvalue_2 (`|GetDataTableRow` "/Game/Blueprints/LootSystem/HealthPack/HealthPackDataTable.HealthPackDataTable" (`|GetArrayItem` _outrownames (`KismetMathLibrary.RandomIntegerInRange` 0 (`KismetArrayLibrary.Array_LastIndex` _outrownames))))
        (:`then`
          (bind (_name _healvalue _healthpack) (break `/Game/Blueprints/LootSystem/HealthPack/HealthPackDataStruct` _returnvalue_2))
          (bind _returnvalue_3 (`|SpawnActorFromClass` _healthpack _returnvalue "AlwaysSpawn" "OverrideRootScale" null _healvalue _name _despawn_time null))
          (return _returnvalue_3))))
    (:`NewEnumerator5`
      (bind _outrownames_2 (`DataTableFunctionLibrary.GetDataTableRowNames` "/Game/Blueprints/LootSystem/Powerup/PowerUpDataTable.PowerUpDataTable"))
      (bind _returnvalue_4 (`|GetDataTableRow` "/Game/Blueprints/LootSystem/Powerup/PowerUpDataTable.PowerUpDataTable" (`|GetArrayItem` _outrownames_2 (`KismetMathLibrary.RandomIntegerInRange` 0 (`KismetArrayLibrary.Array_LastIndex` _outrownames_2))))
        (:`then`
          (bind (_name_2 _duration _powerup) (break `/Game/Blueprints/LootSystem/Powerup/PowerupDataStruct` _returnvalue_4))
          (bind _returnvalue_5 (`|SpawnActorFromClass` _powerup _returnvalue "Undefined" "OverrideRootScale" null _duration _name_2 _despawn_time null))
          (return _returnvalue_5))))))

(fn `Choose Item Type`
  (returns (`Item Type` :type "/Game/Blueprints/LootSystem/LootTypeEnum Enum"))
  (return (select `int` (`KismetMathLibrary.RandomIntegerInRange` 0 5) :`0` "NewEnumerator2" :`1` "NewEnumerator2" :`2` "NewEnumerator5" :`3` "NewEnumerator6" :`4` "NewEnumerator6" :`5` "NewEnumerator6" :!type "/Game/Blueprints/LootSystem/LootTypeEnum Enum")))

(fn `UserConstructionScript`)