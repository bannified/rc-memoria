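; BP_PlayerControllerBase is a base player controller that handles pausing and the pause menu.
; On BeginPlay it creates WBP_PauseMenu, adds it to the viewport at a high Z-order and keeps it collapsed.
; Tab, Escape or the PauseToggle event flips the game's paused state, then shows or collapses the menu, plays an open or close sound and matches mouse cursor visibility to the pause state.
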(event `PauseToggle`
  (bind _returnvalue (`GameplayStatics.IsGamePaused`))
  (`GameplayStatics.SetGamePaused` (not _returnvalue) :!label _label)
  (if _returnvalue
    (bind _pausemenu (`self.PauseMenu`)
      (:`then`
        (`Widget.SetVisibility` _pausemenu "Visible")
        (`GameplayStatics.PlaySound2D` "/Game/Audio/SFX/pauseopen.pauseopen" 1.0 1.0 0.0 null null))
      (:`else`))
    (else
      (bind _pausemenu_2 (`self.PauseMenu`)
        (:`then`
          (`Widget.SetVisibility` _pausemenu_2 "Collapsed")
          (`GameplayStatics.PlaySound2D` "/Game/Audio/SFX/pauseclose.pauseclose" 1.0 1.0 0.0 null null))
        (:`else`))))
  (set `self.bShowMouseCursor` _returnvalue))

(event `Key|Tab` :paused true
  (params (Key :type "Key Structure"))
  (:`Pressed`
    (goto _label)))

(event `Key|Escape` :paused true
  (params (Key :type "Key Structure"))
  (:`Pressed`
    (goto _label)))

(event `self.ReceiveBeginPlay`
  (bind _returnvalue (`|CreateWidget` "/Game/Widgets/GeneralGameplayWidgets/WBP_PauseMenu.WBP_PauseMenu_C" self))
  (bind _output_get (set `self.PauseMenu` _returnvalue))
  (`UserWidget.AddToViewport` _output_get 9999)
  (`Widget.SetVisibility` _output_get "Collapsed"))

(fn `UserConstructionScript`)