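; Base character Blueprint that wires AI behavior, player HUD and damage feedback for units.
; On possession by an AI controller with a behavior tree asset, it runs the tree, enables sight and hearing, and seeds blackboard engagement ranges; otherwise perception is disabled.
; Player possession creates the minimap and binds mana and reload events to the crosshair.
; Instigated health changes spawn randomly offset damage displays, chosen by damage type with a default fallback.
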(event `self.ReceivePossessed`
  (params (NewController :type "Controller Object Reference"))
  (bind _returnvalue (`AIBlueprintHelperLibrary.GetAIController` NewController))
  (bind _aiperception (`self.AIPerception`))
  (bind _unitbehaviortreeasset (`self.UnitBehaviorTreeAsset`)
    (:`then`
      (`/Engine/EditorBlueprintResources/StandardMacros.IsValid` _returnvalue
        (:`Is Valid`
          (`AIController.RunBehaviorTree` _returnvalue _unitbehaviortreeasset)
          (`ActorComponent.SetActive` _aiperception true false)
          (`AIPerceptionComponent.SetSenseEnabled` _aiperception "/Script/AIModule.AISense_Hearing" true)
          (`AIPerceptionComponent.SetSenseEnabled` _aiperception "/Script/AIModule.AISense_Sight" true)
          (`self.InitBlackboardDefaultValues`))
        (:`Is Not Valid`
          (`ActorComponent.SetActive` _aiperception false false :!label _label)
          (`AIPerceptionComponent.SetSenseEnabled` _aiperception "/Script/AIModule.AISense_Hearing" false)
          (`AIPerceptionComponent.SetSenseEnabled` _aiperception "/Script/AIModule.AISense_Sight" false))))
    (:`else`
      (goto _label))))

(event `self.OnReceivePossessedByPlayerControllerBase`
  (params (controllerBase :type "PlayerControllerBase Object Reference"))
  (bind _manacomponent (`self.ManaComponent`))
  ;[1 1 1] Reloading UI Bar & Crosshair Setup
  (add `ManaComponent.ReloadStartEvent` _manacomponent (delegate `ReloadStartEvent_Event_0`))
  (add `ManaComponent.ReloadInterruptEvent` _manacomponent (delegate `ReloadInterruptEvent_Event_0`))
  (add `ManaComponent.ReloadCompleteEvent` _manacomponent (delegate `ReloadCompleteEvent_Event_0`))
  (add `ManaComponent.OnManaChangeEvent` _manacomponent (delegate `OnManaChangeEvent_Event_0`))
  (bind _aswbp_crosshair (cast `/Game/Widgets/WBP_Crosshair` (`self.CrosshairWidget`)))
  (set `/Game/Widgets/WBP_Crosshair.TargetManaComp` (`self.ManaComponent`) _aswbp_crosshair)
  ;[1 1 1] Setup Player UI
  (bind _returnvalue (`|CreateWidget` "/Game/Blueprints/Minimap/Minimap_Widget.Minimap_Widget_C" (`GameplayStatics.GetPlayerController` 0)))
  (bind _output_get (set `self.MinimapWidget` _returnvalue))
  (`UserWidget.AddToViewport` _output_get 0))

(event `OnManaChangeEvent_Event_0`
  (params (character :type "CharacterBase Object Reference") (manaComp :type "ManaComponent Object Reference"))
  ;[1 1 1] Reloading UI Bar & Crosshair Setup
  (bind _aswbp_crosshair (cast `/Game/Widgets/WBP_Crosshair` (`self.CrosshairWidget`)))
  (if (<= (`ManaComponent.CurrentMana` manaComp) 0.0)
    (bind _reloadtextgroup (`/Game/Widgets/WBP_Crosshair.ReloadTextGroup` _aswbp_crosshair))
    (`Widget.SetVisibility` _reloadtextgroup "Visible")
    (else
      (`Widget.SetVisibility` _reloadtextgroup "Hidden"))))

(event `ReloadStartEvent_Event_0`
  (params (character :type "CharacterBase Object Reference") (manaComp :type "ManaComponent Object Reference"))
  ;[1 1 1] Reloading UI Bar & Crosshair Setup
  (bind _aswbp_crosshair (cast `/Game/Widgets/WBP_Crosshair` (`self.CrosshairWidget`)))
  (`Widget.SetVisibility` (`/Game/Widgets/WBP_Crosshair.ReloadBarGroup` _aswbp_crosshair) "Visible")
  (if (<= (`ManaComponent.CurrentMana` (`self.ManaComponent`)) 0.0) :!label _label_2
    (bind _reloadtextgroup (`/Game/Widgets/WBP_Crosshair.ReloadTextGroup` (stale `ReloadInterruptEvent_Event_0` _aswbp_crosshair)))
    (`Widget.SetVisibility` _reloadtextgroup "Visible")
    (else
      (`Widget.SetVisibility` _reloadtextgroup "Hidden"))))

(event `ReloadInterruptEvent_Event_0`
  (params (character :type "CharacterBase Object Reference") (manaComp :type "ManaComponent Object Reference"))
  ;[1 1 1] Reloading UI Bar & Crosshair Setup
  (bind _aswbp_crosshair (cast `/Game/Widgets/WBP_Crosshair` (`self.CrosshairWidget`) :!label _label_3))
  (`Widget.SetVisibility` (`/Game/Widgets/WBP_Crosshair.ReloadBarGroup` _aswbp_crosshair) "Hidden")
  (goto _label_2))

(event `ReloadCompleteEvent_Event_0`
  (params (character :type "CharacterBase Object Reference") (manaComp :type "ManaComponent Object Reference"))
  ;[1 1 1] Reloading UI Bar & Crosshair Setup
  (goto _label_3))

(event `self.OnBeginPlayComplete`
  ;[1 1 1] Common UI Setup
  (bind _aswbp_character_uibase (cast `/Game/Widgets/WBP_CharacterUIBase` (`WidgetComponent.GetUserWidgetObject` (`self.GameplayWidget`)) :!label _label_4)
    (:`then`
      (`/Game/Widgets/WBP_CharacterUIBase.SetupWithCharacterBase` _aswbp_character_uibase self))
    (:`CastFailed`
      (`KismetSystemLibrary.Delay` 0.1)
      (goto _label_4))))

(event `self.HealthComponent.OnHealthChanged`
  (params (HealthComp :type "HealthComponent Object Reference") (health :type "Float (single-precision)") (healthDelta :type "Float (single-precision)") (DamageType :type "DamageType Object Reference") (InstigatedBy :type "Controller Object Reference") (DamageCauser :type "Actor Object Reference"))
  (bind _returnvalue (`Controller.K2_GetPawn` InstigatedBy))
  (bind _returnvalue_2 (`KismetMathLibrary.MakeTransform` (+ (* (`KismetMathLibrary.RandomUnitVector`) 25.0) (`SceneComponent.K2_GetComponentLocation` (`self.DamageDisplayLocation`)))))
  (`/Engine/EditorBlueprintResources/StandardMacros.IsValid` InstigatedBy
    (:`Is Valid`
      (bind _asmemoria_damage_type (cast `MemoriaDamageType` DamageType)
        (:`then`
          (bind _damagedisplaywidgetclass (`MemoriaDamageType.DamageDisplayWidgetClass` _asmemoria_damage_type)
            (:`then`
              (bind _returnvalue_3 (`|SpawnActorFromClass` _damagedisplaywidgetclass _returnvalue_2 "AlwaysSpawn" "OverrideRootScale" self _returnvalue))
              (bind _asbp_default_damage_display (cast `/Game/Widgets/BP_DefaultDamageDisplay` _returnvalue_3))
              (set `/Game/Widgets/BP_DefaultDamageDisplay.Player` self _asbp_default_damage_display)
              (bind _aswbp_damage_display (cast `/Game/Widgets/WBP_DamageDisplay` (`WidgetComponent.GetUserWidgetObject` (`/Game/Widgets/BP_DefaultDamageDisplay.Widget` _asbp_default_damage_display))))
              (set `/Game/Widgets/WBP_DamageDisplay.Value` (`KismetMathLibrary.FTrunc` healthDelta) _aswbp_damage_display))
            (:`else`
              ;[1 1 1] Default Damage Display
              (bind _returnvalue_4 (`|SpawnActorFromClass` "/Game/Widgets/BP_DefaultDamageDisplay.BP_DefaultDamageDisplay_C" _returnvalue_2 "AlwaysSpawn" "OverrideRootScale" self _returnvalue :!label _label_5))
              (set `/Game/Widgets/BP_DefaultDamageDisplay.Player` self _returnvalue_4)
              (bind _aswbp_damage_display_2 (cast `/Game/Widgets/WBP_DamageDisplay` (`WidgetComponent.GetUserWidgetObject` (`/Game/Widgets/BP_DefaultDamageDisplay.Widget` _returnvalue_4))))
              (set `/Game/Widgets/WBP_DamageDisplay.Value` (`KismetMathLibrary.FTrunc` healthDelta) _aswbp_damage_display_2))))
        (:`CastFailed`
          (goto _label_5))))))

(fn `InitBlackboardDefaultValues`
  (bind _returnvalue (`AIBlueprintHelperLibrary.GetBlackboard` null))
  (bind _returnvalue_2 (`MemoriaStaticLibrary.GetModifiableAttributeValue` (`self.MinEngagementRange`)))
  (`BlackboardComponent.SetValueAsFloat` _returnvalue "MinEngagementRange" _returnvalue_2)
  (bind _returnvalue_3 (`MemoriaStaticLibrary.GetModifiableAttributeValue` (`self.MaxEngagementRange`)))
  (`BlackboardComponent.SetValueAsFloat` _returnvalue "MaxEngagementRange" _returnvalue_3))

(fn `SphereOverlapActors`
  (params (`Sphere Pos` :type "Vector Structure") (`Sphere Radius` :type "Float (double-precision)") (`Object Types` :type "Array of EObjectTypeQuery Enum" :default _) (`Actor Class Filter` :type "Object Class Reference") (`Actors to Ignore` :type "Array of Actor Object Reference"))
  (returns (`Out Actors` :type "Array of Actor Object Reference") (HasPassed :type Boolean))
  (bind (_outactors _returnvalue) (`KismetSystemLibrary.SphereOverlapActors` `Sphere Pos` `Sphere Radius` `Object Types` `Actor Class Filter` `Actors to Ignore`))
  (return _outactors _returnvalue))

(fn `UserConstructionScript`)