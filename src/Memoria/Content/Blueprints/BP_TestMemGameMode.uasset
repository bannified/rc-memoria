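; BP_TestMemGameMode is a test game mode that bulk-spawns units, apparently for memory testing.
; On BeginPlay it walks the TestSUAs map, spawning each key's CharacterBase class as many times as the mapped value.
; All units spawn at the first SpawnPoint actor found, adjusted for collision but always spawned.
; Each key's InitializeUnit then sets up the spawned actor.
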(event `self.ReceiveBeginPlay`
  (bind _testsuas (`self.TestSUAs`))
  (bind _outactors (`GameplayStatics.GetAllActorsOfClass` "/Script/Memoria.SpawnPoint"))
  (bind _keys (`BlueprintMapLibrary.Map_Keys` _testsuas))
  (for _array_element _keys
    (for _ (range (`BlueprintMapLibrary.Map_Find` _testsuas _array_element))
      (bind _returnvalue (`|SpawnActorFromClass` (`SpawnUnitAsset.CharacterBase` _array_element) (`KismetMathLibrary.MakeTransform` (`self.K2_GetActorLocation` (`|GetArrayItem` _outactors))) "AdjustIfPossibleButAlwaysSpawn" "OverrideRootScale" null null))
      (`SpawnUnitAsset.InitializeUnit` _array_element _returnvalue))))

(fn `UserConstructionScript`)