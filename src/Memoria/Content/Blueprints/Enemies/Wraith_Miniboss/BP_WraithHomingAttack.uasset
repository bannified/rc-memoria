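; BP_WraithHomingAttack is the Wraith miniboss's homing projectile attack.
; On firing, it rotates the spawned projectile's velocity around the owner's right vector to angle the launch, applying it in local space.
; Projectile movement then homes on the first player's capsule, ignoring the target character passed by the fired event.
; A collision hit spawns a smoke cloud at the impact point.
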(event `self.ReceiveBeginPlay`
  (add `self.ProjectileFired` (delegate `ProjectileFired_Event`)))

(event `ProjectileFired_Event` :!signature `self.ProjectileFired`
  (params (ownerCharacter :type "CharacterBase Object Reference") (targetCharacter :type "Actor Object Reference") (spawnedProjectile :type "ProjectileBase Object Reference"))
  (`/Engine/EditorBlueprintResources/StandardMacros.IsValid` ownerCharacter
    (:`Is Valid`
      (`/Engine/EditorBlueprintResources/StandardMacros.IsValid` spawnedProjectile
        (:`Is Valid`
          (`ProjectileMovementComponent.SetVelocityInLocalSpace` (`ProjectileBase.ProjectileMovement` spawnedProjectile) (`KismetMathLibrary.RotateAngleAxis` (`self.GetVelocity` spawnedProjectile) -60.0 (`self.GetActorRightVector` ownerCharacter)))
          (set `ProjectileMovementComponent.HomingTargetComponent` (`Character.CapsuleComponent` (`GameplayStatics.GetPlayerCharacter` 0)) (`ProjectileBase.ProjectileMovement` spawnedProjectile)))))))

(event `self.CollisionComp.OnComponentHit`
  (params (HitComponent :type "PrimitiveComponent Object Reference") (OtherActor :type "Actor Object Reference") (OtherComp :type "PrimitiveComponent Object Reference") (NormalImpulse :type "Vector Structure") (Hit :type "HitResult Structure (by ref)"))
  (`|SpawnActorFromClass` "/Game/Blueprints/Effects/BP_SmokeCloud.BP_SmokeCloud_C" (`KismetMathLibrary.MakeTransform` Hit_ImpactPoint) "Undefined" "OverrideRootScale" null null))

(fn `UserConstructionScript`)