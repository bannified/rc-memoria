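; Wraith miniboss enemy Blueprint that supplies starting blackboard values for its AI and leaves other behavior to its parent class.
; InitBlackboardValues writes min and max engagement range from modifiable attributes, stores the actor's location as InitialLocation, and sets player pawn 0 as CurrentTarget.
; Possessed, BeginPlay and Destroyed only forward to the parent, and the construction script is empty.
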(event `self.ReceivePossessed`
  (params (NewController :type "Controller Object Reference"))
  (`parent.ReceivePossessed` NewController))

(event `self.ReceiveBeginPlay`
  (`parent.ReceiveBeginPlay`))

(event `self.ReceiveDestroyed`
  (`parent.ReceiveDestroyed`))

(fn `InitBlackboardValues`
  (bind _returnvalue (`AIBlueprintHelperLibrary.GetBlackboard` null))
  (bind _returnvalue_2 (`MemoriaStaticLibrary.GetModifiableAttributeValue` (`self.MinEngagementRange`)))
  (`BlackboardComponent.SetValueAsFloat` _returnvalue "MinEngagementRange" _returnvalue_2)
  (bind _returnvalue_3 (`MemoriaStaticLibrary.GetModifiableAttributeValue` (`self.MaxEngagementRange`)))
  (`BlackboardComponent.SetValueAsFloat` _returnvalue "MaxEngagementRange" _returnvalue_3)
  (`BlackboardComponent.SetValueAsVector` _returnvalue "InitialLocation" (`self.K2_GetActorLocation`))
  (`BlackboardComponent.SetValueAsObject` _returnvalue "CurrentTarget" (`GameplayStatics.GetPlayerPawn` 0)))

(fn `UserConstructionScript`)