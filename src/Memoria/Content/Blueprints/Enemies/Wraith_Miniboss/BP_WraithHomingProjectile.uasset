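; Homing projectile for the Wraith miniboss that leaves a smoke cloud where it hits.
; On a collision component hit, it spawns a BP_SmokeCloud at the impact point and sets that cloud's lifespan from SmokeTime.
; The graphs add no homing, damage or destroy logic; BeginPlay and the construction script only call the parent.
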(event `self.ReceiveBeginPlay`
  (`parent.ReceiveBeginPlay`))

(event `self.CollisionComp.OnComponentHit`
  (params (HitComponent :type "PrimitiveComponent Object Reference") (OtherActor :type "Actor Object Reference") (OtherComp :type "PrimitiveComponent Object Reference") (NormalImpulse :type "Vector Structure") (Hit :type "HitResult Structure (by ref)"))
  (bind _returnvalue (`|SpawnActorFromClass` "/Game/Blueprints/Effects/BP_SmokeCloud.BP_SmokeCloud_C" (`KismetMathLibrary.MakeTransform` Hit_ImpactPoint) "Undefined" "OverrideRootScale" null null))
  (`self.SetLifeSpan` _returnvalue (`self.SmokeTime`)))

(fn `UserConstructionScript`
  (`parent.UserConstructionScript`))