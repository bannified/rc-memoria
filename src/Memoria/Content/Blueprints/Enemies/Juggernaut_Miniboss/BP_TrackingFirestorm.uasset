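; Tracking Firestorm attack for the Juggernaut miniboss, which launches homing projectiles from the boss's fins.
; On setup it binds to the Juggernaut's fin attack and taunt events, and AttackStart plays the fin attack montage.
; The fin trigger spawns a projectile at each configured socket, homing on the blackboard's CurrentTarget capsule, with muzzle flare and fire sound.
; The taunt event plays a sound attached to the head.
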(event `self.OnReceiveSetupWithCharacter`
  (params (characterBase :type "CharacterBase Object Reference"))
  (bind _asbp_juggernaut (cast `/Game/Blueprints/Enemies/Juggernaut_Miniboss/BP_Juggernaut` characterBase))
  (add `/Game/Blueprints/Enemies/Juggernaut_Miniboss/BP_Juggernaut.FinAttackEvent` _asbp_juggernaut (delegate `FinAttackTrigger`))
  (add `/Game/Blueprints/Enemies/Juggernaut_Miniboss/BP_Juggernaut.FinAttackTauntEvent` _asbp_juggernaut (delegate `FinAttackTaunt`)))

(event `FinAttackTrigger`
  (`self.FireFromFins`))

(event `FinAttackTaunt`
  (`GameplayStatics.SpawnSoundAttached` (`self.TauntSoundCue`) (`Character.Mesh` (`self.ownerCharacter`)) "FX_Head" (0.0 0.0 0.0) (struct) "KeepRelativeOffset" false 1.0 1.0 0.0 null null))

(event `self.ReceiveAttackStart`
  (`Character.PlayAnimMontage` (`self.ownerCharacter`) "/Game/Blueprints/Enemies/Juggernaut_Miniboss/AM_FinAttack.AM_FinAttack" 1.0 "None"))

(fn `FireFromFins`
  (locals (TargetCharacter :type "CharacterBase Object Reference"))
  (bind _ownercharacter (`self.ownerCharacter`))
  (bind _mesh (`Character.Mesh` _ownercharacter))
  (bind _mesh_2 (`Character.Mesh` (`self.ownerCharacter`)))
  (bind _ascharacter_base (cast `CharacterBase` (`BlackboardComponent.GetValueAsObject` (`AIBlueprintHelperLibrary.GetBlackboard` (`self.ownerCharacter`)) "CurrentTarget")))
  (set `local.TargetCharacter` _ascharacter_base)
  (for _array_element (`self.SocketNames`)
    (bind _returnvalue (`|SpawnActorFromClass` (`self.ProjectileClass`) (`KismetMathLibrary.MakeTransform` (`SceneComponent.GetSocketLocation` _mesh _array_element) (`SceneComponent.GetSocketRotation` _mesh _array_element)) "AdjustIfPossibleButAlwaysSpawn" "OverrideRootScale" _ownercharacter _ownercharacter))
    (`ProjectileBase.SetupWithCharacter` _returnvalue _ownercharacter)
    (set `ProjectileMovementComponent.HomingTargetComponent` (`Character.CapsuleComponent` (`local.TargetCharacter`)) (`ProjectileBase.ProjectileMovement` _returnvalue))
    (`GameplayStatics.SpawnEmitterAttached` (`self.MuzzleFlare`) _mesh_2 _array_element (0.0 0.0 0.0) (struct) (1.0 1.0 1.0) "KeepRelativeOffset" true "AutoRelease")
    (`GameplayStatics.SpawnSoundAttached` (`self.FireSound`) _mesh_2 _array_element (0.0 0.0 0.0) (struct) "KeepRelativeOffset" false 1.0 1.0 0.0 null null)))

(fn `UserConstructionScript`)