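; Homing firestorm actor for the Juggernaut miniboss that leaves a flame area on the ground when destroyed.
; On destruction it line-traces against WorldStatic, with the end point computed by multiplying its location by a scaled down vector rather than adding it.
; A hit spawns BP_FlameArea at the impact point, passing on owner, controller, scale, lifespan and damage per interval.
; Homing behavior is not defined in these graphs.
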(event `self.ReceiveBeginPlay`
  (`parent.ReceiveBeginPlay`)
  (add `self.OnDestroyed` (delegate `OnDestroyed_Event_0`)))

(event `OnDestroyed_Event_0` :!signature `self.OnDestroyed`
  (params (DestroyedActor :type "Actor Object Reference"))
  (bind _returnvalue (`self.K2_GetActorLocation` DestroyedActor))
  (bind (_outhit _returnvalue_2) (`KismetSystemLibrary.LineTraceSingleForObjects` _returnvalue (* _returnvalue (* (`KismetMathLibrary.Vector_Down`) 200.0)) (`|MakeArray` "ObjectTypeQuery1" :!type "EObjectTypeQuery Enum")))
  (if _returnvalue_2
    (bind _returnvalue_3 (`|SpawnActorFromClass` "/Game/Blueprints/Enemies/Juggernaut_Miniboss/BP_FlameArea.BP_FlameArea_C" (`KismetMathLibrary.MakeTransform` (`.ImpactPoint` (`GameplayStatics.BreakHitResult` _outhit)) (struct) (`KismetMathLibrary.Conv_Vector2DToVector` (`self.FlameAreaScale`) 1.0)) "Undefined" "OverrideRootScale" (`self.OwningActor`) null))
    (set `/Game/Blueprints/Enemies/Juggernaut_Miniboss/BP_FlameArea.OwningController` (`self.OwningController`) _returnvalue_3)
    (`self.SetLifeSpan` _returnvalue_3 (`self.FlameAreaLifespan`))
    (set `/Game/Blueprints/Enemies/Juggernaut_Miniboss/BP_FlameArea.DamagePerInterval` (`self.FlameAreaDamagePerInterval`) _returnvalue_3)))

(fn `UserConstructionScript`
  (`parent.UserConstructionScript`))