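; Juggernaut miniboss Blueprint that shows a named boss health bar on the player's HUD.
; On BeginPlay it creates a WBP_BossHPBarDisplay bound to itself and adds it to player 0's HUD as a highlight widget.
; On Destroyed it removes the widget held in HPBarWidget, which this graph never assigns.
; Tick, overlap and construction script add no logic of their own.
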(event `self.ReceiveBeginPlay`
  (`parent.ReceiveBeginPlay`)
  (bind _asbp_player_character_base (cast `/Game/Blueprints/BP_PlayerCharacterBase` (`GameplayStatics.GetPlayerPawn` 0)))
  (bind _returnvalue (`self.GetPlayerControllerBase` _asbp_player_character_base))
  (bind _playerhudwidget (`/Game/Blueprints/BP_PlayerCharacterBase.PlayerHUDWidget` _asbp_player_character_base)
    (:`then`
      (bind _returnvalue_2 (`|CreateWidget` "/Game/Widgets/MinionWidgets/WBP_BossHPBarDisplay.WBP_BossHPBarDisplay_C" _returnvalue))
      (`/Game/Widgets/MinionWidgets/WBP_BossHPBarDisplay.SetupWithCharacter` _returnvalue_2 self "Juggernaut")
      (`/Game/Widgets/GeneralGameplayWidgets/WBP_PlayerHUD.AddHighlightWidget` _playerhudwidget _returnvalue_2))
    (:`else`)))

(event `self.ReceiveDestroyed`
  (bind _hpbarwidget (`self.HPBarWidget`)
    (:`then`
      (bind _asbp_player_character_base (cast `/Game/Blueprints/BP_PlayerCharacterBase` (`GameplayStatics.GetPlayerPawn` 0)))
      (bind _playerhudwidget (`/Game/Blueprints/BP_PlayerCharacterBase.PlayerHUDWidget` _asbp_player_character_base)
        (:`then`
          (`/Game/Widgets/GeneralGameplayWidgets/WBP_PlayerHUD.RemoveHighlightWidget` _playerhudwidget _hpbarwidget))
        (:`else`)))
    (:`else`)))

(fn `UserConstructionScript`
  (`parent.UserConstructionScript`))