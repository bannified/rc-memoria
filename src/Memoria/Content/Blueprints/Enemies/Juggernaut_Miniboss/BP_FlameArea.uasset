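; BP_FlameArea is a damage-over-time hazard in the Juggernaut miniboss enemy folder that hurts characters standing inside its cylinder volume.
; Cylinder overlap events add and remove BP_CharacterBase actors in an AffectedActors list.
; A looping timer started on BeginPlay applies Memoria-type damage to every listed character at a set interval, credited to the owning controller.
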(event `self.Cylinder.OnComponentBeginOverlap`
  (params (OverlappedComponent :type "PrimitiveComponent Object Reference") (OtherActor :type "Actor Object Reference") (OtherComp :type "PrimitiveComponent Object Reference") (OtherBodyIndex :type Integer) (bFromSweep :type Boolean) (SweepResult :type "HitResult Structure (by ref)"))
  (bind _asbp_character_base (cast `/Game/Blueprints/BP_CharacterBase` OtherActor))
  (`KismetArrayLibrary.Array_Add` (`self.AffectedActors`) _asbp_character_base))

(event `self.Cylinder.OnComponentEndOverlap`
  (params (OverlappedComponent :type "PrimitiveComponent Object Reference") (OtherActor :type "Actor Object Reference") (OtherComp :type "PrimitiveComponent Object Reference") (OtherBodyIndex :type Integer))
  (bind _asbp_character_base (cast `/Game/Blueprints/BP_CharacterBase` OtherActor))
  (`KismetArrayLibrary.Array_RemoveItem` (`self.AffectedActors`) _asbp_character_base))

(event `self.ReceiveBeginPlay`
  (`KismetSystemLibrary.K2_SetTimerDelegate` (delegate `DamageEvent`) (`self.IntervalDuration`) true))

(event `DamageEvent`
  (for _array_element (`self.AffectedActors`)
    (`GameplayStatics.ApplyDamage` _array_element (`self.DamagePerInterval`) (`self.OwningController`) self "/Game/Blueprints/DamageTypes/BP_MemoriaDamageType.BP_MemoriaDamageType_C")))

(fn `UserConstructionScript`)