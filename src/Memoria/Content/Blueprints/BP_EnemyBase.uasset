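; Base enemy Blueprint that provides shared AI targeting, a minimap marker and death rewards.
; On BeginPlay it spawns and attaches an overhead sprite as the minimap icon.
; AI perception updates the blackboard's current target and last-seen location, and a helper function copies engagement-range attributes into the blackboard.
; On destruction it removes the icon, notifies the player of the kill and spawns a timed item drop driven by enemy loot tables.
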(event `self.OnReceivePossessedByPlayerControllerBase`
  (params (controllerBase :type "PlayerControllerBase Object Reference"))
  (`parent.OnReceivePossessedByPlayerControllerBase` controllerBase))

(event `self.ReceivePossessed`
  (params (NewController :type "Controller Object Reference"))
  (`parent.ReceivePossessed` NewController))

(event `self.ReceiveBeginPlay`
  (`parent.ReceiveBeginPlay`)
  ;[1 1 1] Minimap icon setup
  (`self.InitMinimapEnemyIcon`))

(event `self.ReceiveDestroyed`
  ;[1 1 1] Minimap icon setup
  (`self.K2_DestroyActor` (`self.EnemyIcon`))
  ;[1 1 1] Increment player kill count when enemy dies
  (bind _asbp_player_character_base (cast `/Game/Blueprints/BP_PlayerCharacterBase` (`GameplayStatics.GetPlayerPawn` 0)))
  (`/Game/Blueprints/BP_PlayerCharacterBase.OnEnemyKilled` _asbp_player_character_base)
  (`|SpawnActorFromClass` "/Game/Blueprints/LootSystem/BP_ItemSpawn.BP_ItemSpawn_C" (`KismetMathLibrary.Conv_VectorToTransform` (`KismetMathLibrary.MakeVector` (.x (`self.K2_GetActorLocation`)) (.y (`self.K2_GetActorLocation`)) (- (.z (`self.K2_GetActorLocation`)) 50.0))) "AdjustIfPossibleButAlwaysSpawn" "OverrideRootScale" null 60.0 "/Game/Blueprints/LootSystem/DT_ItemType_EnemyBase.DT_ItemType_EnemyBase" "/Game/Blueprints/LootSystem/HealthPack/DT_HealthPack_EnemyBase.DT_HealthPack_EnemyBase" "/Game/Blueprints/LootSystem/Powerup/DT_PowerUp_EnemyBase.DT_PowerUp_EnemyBase" null))

(event `self.AIPerception.OnTargetPerceptionUpdated`
  (params (Actor :type "Actor Object Reference") (Stimulus :type "AIStimulus Structure"))
  (bind _returnvalue (`AIBlueprintHelperLibrary.GetBlackboard` null))
  (bind _returnvalue_2 (`BlackboardComponent.GetValueAsObject` _returnvalue "CurrentTarget"))
  ;[1 1 1] AIPerception-related
  (if Stimulus_bSuccessfullySensed
    (`BlackboardComponent.SetValueAsObject` _returnvalue "CurrentTarget" Actor)
    (cast `Actor` _returnvalue_2)
    (elif (== Actor _returnvalue_2)
      (`BlackboardComponent.SetValueAsVector` _returnvalue "CurrentTargetLastSeenLocation" (`self.K2_GetActorLocation` Actor))
      (`BlackboardComponent.ClearValue` _returnvalue "CurrentTarget"))))

(fn `InitDefaultBlackboardValues`
  (bind _returnvalue (`AIBlueprintHelperLibrary.GetBlackboard` null))
  (bind _returnvalue_2 (`MemoriaStaticLibrary.GetModifiableAttributeValue` (`self.MinEngagementRange`)))
  (`BlackboardComponent.SetValueAsFloat` _returnvalue "MinEngagementRange" _returnvalue_2)
  (bind _returnvalue_3 (`MemoriaStaticLibrary.GetModifiableAttributeValue` (`self.MaxEngagementRange`)))
  (`BlackboardComponent.SetValueAsFloat` _returnvalue "MaxEngagementRange" _returnvalue_3))

(fn `InitMinimapEnemyIcon`
  (bind _returnvalue (`|SpawnActorFromClass` "/Game/Blueprints/Minimap/BP_Sprite.BP_Sprite_C" (`KismetMathLibrary.MakeTransform` (+ (`self.K2_GetActorLocation`) (0.0 0.0 1000.0)) (struct :`Roll` -90.0) (0.15 0.15 0.15)) "Undefined" "OverrideRootScale" null null))
  (bind _output_get (set `self.EnemyIcon` _returnvalue))
  (`self.SetOwner` _output_get (`GameplayStatics.GetPlayerPawn` 0))
  (`self.K2_AttachToActor` (`self.EnemyIcon`) self "None" "KeepWorld" "KeepWorld" "KeepWorld" false))

(fn `UserConstructionScript`)