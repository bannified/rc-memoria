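; BP_Sentry is a sentry Blueprint that creates and reveals a Projectile_Sentry for a character.
; On character setup it spawns the projectile with the capsule's rotation, at a position made by scaling the capsule's world X and Z rather than adding an offset.
; AttackStart only makes that projectile's root component visible.
; Code to reposition the projectile exists but is unconnected, and BeginPlay and Tick are empty.
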(event `self.ReceiveTick`
  (params (DeltaSeconds :type "Float (single-precision)")))

(event `self.OnReceiveSetupWithCharacter`
  (params (characterBase :type "CharacterBase Object Reference"))
  (bind _returnvalue (`|SpawnActorFromClass` "/Game/Blueprints/Characters/Projectile_Sentry.Projectile_Sentry_C" (`KismetMathLibrary.MakeTransform` (`KismetMathLibrary.MakeVector` (* (.x (`SceneComponent.K2_GetComponentLocation` (`Character.CapsuleComponent` characterBase))) 1.25) (* (.y (`SceneComponent.K2_GetComponentLocation` (`Character.CapsuleComponent` characterBase))) 1.0) (* (.z (`SceneComponent.K2_GetComponentLocation` (`Character.CapsuleComponent` characterBase))) 1.6)) (`SceneComponent.K2_GetComponentRotation` (`Character.CapsuleComponent` characterBase)) (1.0 1.0 1.0)) "Undefined" "OverrideRootScale" null null)))

(event `self.ReceiveAttackStart`
  (`SceneComponent.SetVisibility` (`Actor.RootComponent` (stale `self.OnReceiveSetupWithCharacter` _returnvalue)) true false))

(fn `UserConstructionScript`
  (`parent.UserConstructionScript`))