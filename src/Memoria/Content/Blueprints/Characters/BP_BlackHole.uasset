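; Black hole ability for a character that previews an aimed throw and spawns a temporary black hole where it would land.
; Every tick it predicts a projectile arc from the character's camera and moves a marker actor, spawned on setup, to the trace's end point.
; Attack start shows the debug arc and marker sphere.
; Attack end hides both, spawns the BlackHole at that point and destroys it after a short delay.
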(event `self.ReceiveTick`
  (params (DeltaSeconds :type "Float (single-precision)"))
  (bind _returnvalue (`SceneComponent.GetForwardVector` (`CharacterBase.MainCamera` (stale `self.OnReceiveSetupWithCharacter` characterBase))))
  (bind (_outhit _outpathpositions _outlasttracedestination) (`GameplayStatics.Blueprint_PredictProjectilePath_ByTraceChannel` :`StartPos` (+ (`self.K2_GetActorLocation` (stale `self.OnReceiveSetupWithCharacter` characterBase)) (* _returnvalue 75.0)) :`LaunchVelocity` (* _returnvalue 2500.0) :`DrawDebugType` (`self.NewVar_0`) :`DrawDebugTime` 0.02))
  (`SceneComponent.K2_SetWorldLocation` (`Actor.RootComponent` (stale `self.OnReceiveSetupWithCharacter` _returnvalue)) _outlasttracedestination false false))

(event `self.OnReceiveSetupWithCharacter`
  (params (characterBase :type "CharacterBase Object Reference"))
  (bind _returnvalue (`|SpawnActorFromClass` "/Game/Blueprints/Projectiles/Predicted_Projectile.Predicted_Projectile_C" (`KismetMathLibrary.Conv_VectorToTransform` (stale `self.ReceiveTick` _outlasttracedestination)) "Undefined" "OverrideRootScale" null null))
  (`SceneComponent.SetVisibility` (`/Game/Blueprints/Projectiles/Predicted_Projectile.Sphere` _returnvalue) false false))

(event `self.ReceiveAttackStart`
  (set `self.NewVar_0` "ForOneFrame")
  (`SceneComponent.SetVisibility` (`/Game/Blueprints/Projectiles/Predicted_Projectile.Sphere` (stale `self.OnReceiveSetupWithCharacter` _returnvalue)) true false))

(event `self.ReceiveAttackEnd`
  (set `self.NewVar_0` "None")
  (`SceneComponent.SetVisibility` (`/Game/Blueprints/Projectiles/Predicted_Projectile.Sphere` (stale `self.OnReceiveSetupWithCharacter` _returnvalue)) false false)
  (bind _returnvalue (`|SpawnActorFromClass` "/Game/Blueprints/Projectiles/BlackHole.BlackHole_C" (`KismetMathLibrary.Conv_VectorToTransform` (stale `self.ReceiveTick` _outlasttracedestination)) "Undefined" "OverrideRootScale" null null))
  (`KismetSystemLibrary.Delay` 3.0)
  (`self.K2_DestroyActor` _returnvalue))

(fn `UserConstructionScript`
  (`parent.UserConstructionScript`))