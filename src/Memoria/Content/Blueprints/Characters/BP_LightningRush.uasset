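; Lightning Rush character attack that launches the character along its facing and damages non-friendly pawns near the starting position.
; On AttackStart it runs one box overlap, offset toward the camera's aim point but world-axis aligned, and draws a debug box.
; Each enemy hit takes damage and triggers a temporary radial force impulse at the character.
; The cleanup Delay sits inside the loop, so multiple hits leave components undestroyed.
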(event `self.OnReceiveSetupWithCharacter`
  (params (characterBase :type "CharacterBase Object Reference")))

(event `self.ReceiveAttackStart`
  (bind _ownercharacter (`self.ownerCharacter`))
  (bind _rootcomponent (`Actor.RootComponent` (stale `self.OnReceiveSetupWithCharacter` characterBase)))
  (`Character.LaunchCharacter` (stale `self.OnReceiveSetupWithCharacter` characterBase) (* (`SceneComponent.GetForwardVector` _rootcomponent) 4000) false false)
  (bind _maincamera (`CharacterBase.MainCamera` (stale `self.OnReceiveSetupWithCharacter` characterBase)))
  (bind (_returnvalue_x _returnvalue_y _returnvalue_z) (`KismetMathLibrary.BreakVector` (`SceneComponent.K2_GetComponentLocation` (`Actor.RootComponent` (stale `self.OnReceiveSetupWithCharacter` characterBase)))))
  (bind _returnvalue (`KismetMathLibrary.MakeVector` _returnvalue_x _returnvalue_y (+ _returnvalue_z (`.OutHalfHeight` (`CapsuleComponent.GetScaledCapsuleSize` (`Character.CapsuleComponent` (stale `self.OnReceiveSetupWithCharacter` characterBase)))))))
  (bind _returnvalue_2 (+ (* (`KismetMathLibrary.Normal` (- (+ (* (`KismetMathLibrary.GetForwardVector` (`SceneComponent.K2_GetComponentRotation` _maincamera)) 10000.0) (`SceneComponent.K2_GetComponentLocation` _maincamera)) (`SceneComponent.K2_GetComponentLocation` _rootcomponent))) 100.0) _returnvalue))
  (bind (_outactors _returnvalue_3) (`KismetSystemLibrary.BoxOverlapActors` _returnvalue_2 (500.0 100.0 50.0) (`|MakeArray` "ObjectTypeQuery3" :!type "EObjectTypeQuery Enum")))
  (`KismetSystemLibrary.DrawDebugBox` _returnvalue_2 (500.0 100.0 50.0) (struct :`A` 1.0) (struct) 0.0 3.0)
  (if _returnvalue_3
    (for _array_element _outactors
      (bind _returnvalue_4 (`HealthComponent.IsFriendly` _array_element _ownercharacter))
      (if (not _returnvalue_4)
        (`GameplayStatics.ApplyDamage` _array_element 20.0 (`Pawn.GetController` _ownercharacter) _ownercharacter "/Script/Engine.DamageType")
        (bind _returnvalue_5 (`AddComponent|NODE_AddRadialForceComponent-0` :`RelativeTransform` (`KismetMathLibrary.Conv_VectorToTransform` _returnvalue)))
        (`RadialForceComponent.FireImpulse` _returnvalue_5)
        (`KismetSystemLibrary.Delay` 1.0)
        (`ActorComponent.K2_DestroyComponent` _returnvalue_5)))))

(fn `UserConstructionScript`
  (`parent.UserConstructionScript`))