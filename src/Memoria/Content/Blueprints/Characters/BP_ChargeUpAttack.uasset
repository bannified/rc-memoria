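; BP_ChargeUpAttack is a character's charge-up attack Blueprint that handles the looping charge sound.
; On BeginPlay it binds handlers to the charge begin, max and release events.
; Charge begin spawns the loop sound attached to the owner's weapon mesh at the muzzle socket and stores the audio component.
; Reaching max charge or releasing shares one path that stops and destroys that component if it is valid.
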(event `self.ReceiveBeginPlay`
  (add `self.OnChargeBegin` (delegate `OnChargeBegin_Event`))
  (add `self.OnChargeMax` (delegate `OnChargeMax_Event`))
  (add `self.OnChargeRelease` (delegate `OnChargeRelease_Event`)))

(event `OnChargeBegin_Event` :!signature `self.OnChargeBegin`
  (params (attack :type "ChargeUpProjectileAttack Object Reference"))
  (bind _returnvalue (`CharacterBase.GetWeaponMeshComponent` (`self.ownerCharacter`)))
  (bind _returnvalue_2 (`GameplayStatics.SpawnSoundAttached` (`self.ChargingLoopSound`) _returnvalue (`self.MuzzleSocketName`) (0.0 0.0 0.0) (struct) "SnapToTargetIncludingScale" false 1.0 1.0 0.0 null null))
  (set `self.LoopAudioComp` _returnvalue_2))

(event `OnChargeMax_Event` :!signature `self.OnChargeMax`
  (params (attack :type "ChargeUpProjectileAttack Object Reference"))
  (bind _loopaudiocomp (`self.LoopAudioComp` :!label _label)
    (:`then`
      (`AudioComponent.Stop` _loopaudiocomp)
      (`ActorComponent.K2_DestroyComponent` _loopaudiocomp))
    (:`else`)))

(event `OnChargeRelease_Event` :!signature `self.OnChargeRelease`
  (params (attack :type "ChargeUpProjectileAttack Object Reference"))
  (goto _label))

(fn `UserConstructionScript`)