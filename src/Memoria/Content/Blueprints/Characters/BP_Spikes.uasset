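; BP_Spikes is a character attack that surrounds its owner with a spawned Spikes actor.
; AttackStart spawns Spikes scaled by SpikesSize, offset half a capsule half-height below center, and attaches it to the owner's capsule to follow the character.
; It sets the actor's lifespan from Duration and passes on DamagePerTick.
; An unconnected branch for manually moving the spikes to the capsule never runs.
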(event `self.ReceiveTick`
  (params (DeltaSeconds :type "Float (single-precision)")))

(event `self.OnReceiveSetupWithCharacter`
  (params (characterBase :type "CharacterBase Object Reference")))

(event `self.ReceiveAttackStart`
  (bind _ownercharacter (`self.ownerCharacter`))
  (bind _spikessize (`self.SpikesSize`))
  (bind _capsulecomponent (`Character.CapsuleComponent` _ownercharacter))
  (bind _returnvalue (`|SpawnActorFromClass` "/Game/Blueprints/Characters/Spikes.Spikes_C" (`KismetMathLibrary.MakeTransform` (`KismetMathLibrary.MakeVector` 0.0 0.0 (* (`CapsuleComponent.GetScaledCapsuleHalfHeight` _capsulecomponent) -0.5)) (struct) (`KismetMathLibrary.MakeVector` _spikessize _spikessize _spikessize)) "AlwaysSpawn" "OverrideRootScale" _ownercharacter _ownercharacter))
  (`self.K2_AttachToComponent` _returnvalue _capsulecomponent "None" "KeepRelative" "KeepRelative" "KeepRelative" true)
  (`self.SetLifeSpan` _returnvalue (`self.Duration`))
  (set `/Game/Blueprints/Characters/Spikes.DamagePerTick` (`self.DamagePerTick`) _returnvalue))

(fn `UserConstructionScript`
  (`parent.UserConstructionScript`))