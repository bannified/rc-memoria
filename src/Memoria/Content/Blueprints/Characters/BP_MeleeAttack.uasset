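; Melee attack for BP_CharacterBase that plays the "Melee" montage and damages non-friendly characters.
; AttackStart locks yaw to the controller and gathers targets with a camera-aimed box overlap as the montage starts, also drawing a debug box.
; The trigger anim notify damages stored targets still within MeleeRange, combining attack damage with the owner's base and multiplier stats.
; The end notify calls the character's AttackEnd, and this attack's AttackEnd releases the yaw lock.
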(event `OnAttackEnd_AnimNotify_Event_0`
  (params (Character :type "CharacterBase Object Reference"))
  (`CharacterBase.AttackEnd` Character (`self.AttackIndex`)))

(event `self.OnReceiveSetupWithCharacter`
  (params (characterBase :type "CharacterBase Object Reference"))
  (add `CharacterBase.OnAttackTrigger_AnimNotify` characterBase (delegate `OnAttackTrigger_AnimNotify_Event_0`))
  (add `CharacterBase.OnAttackEnd_AnimNotify` characterBase (delegate `OnAttackEnd_AnimNotify_Event_0`)))

(event `OnAttackTrigger_AnimNotify_Event_0`
  (params (Character :type "CharacterBase Object Reference"))
  (bind _ownercharacter (`self.ownerCharacter`))
  (cast `/Game/Blueprints/BP_CharacterBase` Character)
  (bind _finaldamage (`self.GetFinalDamage`))
  (for _array_element (`self.AcquiredTargets`)
    (`/Engine/EditorBlueprintResources/StandardMacros.IsValid` _array_element
      (:`Is Valid`
        (if (<= (`KismetMathLibrary.Vector_Distance` (`self.K2_GetActorLocation` (`self.ownerCharacter`)) (`self.K2_GetActorLocation` _array_element)) (`self.MeleeRange`))
          (`GameplayStatics.ApplyDamage` _array_element _finaldamage (`Pawn.GetController` _ownercharacter) _ownercharacter "/Script/Engine.DamageType"))))))

(event `self.ReceiveAttackStart`
  (bind _ownercharacter (`self.ownerCharacter`))
  (bind _attackcollisionboxextent (`self.AttackCollisionBoxExtent`))
  (bind _ownercharacter_2 (`self.ownerCharacter`))
  (bind _maincamera (`CharacterBase.MainCamera` _ownercharacter_2))
  (bind (_returnvalue_x _returnvalue_y _returnvalue_z) (`KismetMathLibrary.BreakVector` (`SceneComponent.K2_GetComponentLocation` (`Character.Mesh` _ownercharacter_2))))
  (bind _returnvalue (+ (* (`KismetMathLibrary.Normal` (- (+ (* (`KismetMathLibrary.GetForwardVector` (`SceneComponent.K2_GetComponentRotation` _maincamera)) 10000.0) (`SceneComponent.K2_GetComponentLocation` _maincamera)) (`self.K2_GetActorLocation` _ownercharacter_2))) (`self.AttackCollisionBoxOffsetDistance`)) (`KismetMathLibrary.MakeVector` _returnvalue_x _returnvalue_y (+ _returnvalue_z (`.OutHalfHeight` (`CapsuleComponent.GetScaledCapsuleSize` (`Character.CapsuleComponent` _ownercharacter_2)))))))
  (set `Pawn.bUseControllerRotationYaw` true _ownercharacter)
  (cast `/Game/Blueprints/BP_CharacterBase` _ownercharacter)
  (bind _returnvalue_2 (`CharacterBase.GetAnimWithName` _ownercharacter "Melee"))
  (`/Engine/EditorBlueprintResources/StandardMacros.IsValid` _returnvalue_2
    (:`Is Valid`
      (`|PlayMontage` (`Character.Mesh` _ownercharacter) _returnvalue_2
        (:`then`
          (`KismetArrayLibrary.Array_Clear` (`self.AcquiredTargets`))
          (bind (_outactors _returnvalue_3) (`KismetSystemLibrary.BoxOverlapActors` _returnvalue _attackcollisionboxextent (`|MakeArray` "ObjectTypeQuery3" :!type "EObjectTypeQuery Enum") "/Game/Blueprints/BP_CharacterBase.BP_CharacterBase_C" (`|MakeArray` _ownercharacter_2 :!type "Actor Object Reference")))
          (`KismetSystemLibrary.DrawDebugBox` _returnvalue _attackcollisionboxextent (struct :`G` 1.0 :`B` 0.176688 :`A` 1.0) (struct) 5.0 5.0)
          (if _returnvalue_3
            (for _array_element _outactors
              (bind _returnvalue_4 (`HealthComponent.IsFriendly` _array_element (`self.ownerCharacter`)))
              (if (not _returnvalue_4)
                (`KismetArrayLibrary.Array_Add` (`self.AcquiredTargets`) _array_element)))))))))

(event `self.ReceiveAttackEnd`
  (set `Pawn.bUseControllerRotationYaw` false (`self.ownerCharacter`)))

(fn `GetFinalDamage`
  (returns (FinalDamage :type "Float (double-precision)"))
  (bind _returnvalue (`MemoriaStaticLibrary.GetModifiableAttributeValue` (`self.Damage`)))
  (bind _ownercharacter (`self.ownerCharacter`)
    (:`then`
      (bind _returnvalue_2 (`MemoriaStaticLibrary.GetModifiableAttributeValue` (`CharacterBase.StatBaseDamage` _ownercharacter)))
      (bind _returnvalue_3 (`MemoriaStaticLibrary.GetModifiableAttributeValue` (`CharacterBase.StatDamageMultiplier` _ownercharacter)))
      (return (* (+ _returnvalue_2 _returnvalue) _returnvalue_3)))
    (:`else`
      (return _returnvalue))))

(fn `UserConstructionScript`)