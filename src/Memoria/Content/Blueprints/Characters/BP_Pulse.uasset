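; BP_Pulse is a character attack that fires a short-lived Pulse actor from the owning character.
; AttackStart spawns the Pulse slightly ahead of the character's location along the main camera's forward vector, matching the camera's rotation.
; After a brief delay it destroys that spawned actor; the setup event and construction script add no logic of their own.
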(event `self.OnReceiveSetupWithCharacter`
  (params (characterBase :type "CharacterBase Object Reference")))

(event `self.ReceiveAttackStart`
  (bind _maincamera (`CharacterBase.MainCamera` (stale `self.OnReceiveSetupWithCharacter` characterBase)))
  (bind _returnvalue (`|SpawnActorFromClass` "/Game/Blueprints/Projectiles/Pulse.Pulse_C" (`KismetMathLibrary.MakeTransform` (+ (`self.K2_GetActorLocation` (stale `self.OnReceiveSetupWithCharacter` characterBase)) (* (`SceneComponent.GetForwardVector` _maincamera) 40.0)) (`SceneComponent.K2_GetComponentRotation` _maincamera)) "Undefined" "OverrideRootScale" null null))
  (`KismetSystemLibrary.Delay` 0.7)
  (`self.K2_DestroyActor` _returnvalue))

(fn `UserConstructionScript`
  (`parent.UserConstructionScript`))