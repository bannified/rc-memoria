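; Spikes is a hazard that damages and knocks back enemies within its Sphere component.
; Every Tick it queries the sphere for overlapping BP_EnemyBase actors and applies fixed damage, with the first player controller as damage causer.
; It also pushes each enemy opposite its own forward vector with a large movement impulse.
; Damage and impulse repeat each frame during overlap, without delta-time scaling.
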(event `self.ReceiveTick`
  (params (DeltaSeconds :type "Float (single-precision)"))
  (for _array_element (`PrimitiveComponent.GetOverlappingActors` (`self.Sphere`) "/Game/Blueprints/BP_EnemyBase.BP_EnemyBase_C")
    (bind _asbp_enemy_base (cast `/Game/Blueprints/BP_EnemyBase` _array_element))
    (`GameplayStatics.ApplyDamage` _asbp_enemy_base 10.0 null (`GameplayStatics.GetPlayerController` 0))
    (`CharacterMovementComponent.AddImpulse` (`Character.CharacterMovement` _asbp_enemy_base) (* (`KismetMathLibrary.NegateVector` (`SceneComponent.GetForwardVector` (`Actor.RootComponent` _array_element))) 300000.0) false)))

(fn `UserConstructionScript`)