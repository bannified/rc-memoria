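; BP_TestDummy1 is a test pawn that defers possession, begin play and destruction handling to its parent class.
; Its ShootProjectile function spawns a projectile at the actor's location, aimed along the control rotation, with itself as owner and instigator.
; The projectile receives the pawn's team number, owning actor and controller, and its ignored-actor list is reset to just the shooter.
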(event `self.ReceivePossessed`
  (params (NewController :type "Controller Object Reference"))
  (`parent.ReceivePossessed` NewController))

(event `self.ReceiveBeginPlay`
  (`parent.ReceiveBeginPlay`))

(event `self.ReceiveDestroyed`
  (`parent.ReceiveDestroyed`))

(fn `ShootProjectile`
  (bind _returnvalue (`|SpawnActorFromClass` (`self.Projectile`) (`KismetMathLibrary.MakeTransform` (`self.K2_GetActorLocation`) (`self.GetControlRotation`)) "AlwaysSpawn" "OverrideRootScale" self self))
  (bind _returnvalue_2 (`self.GetTeamNumber`))
  (set `ProjectileBase.TeamNumber` (`KismetMathLibrary.Conv_IntToByte` _returnvalue_2) _returnvalue)
  (set `ProjectileBase.OwningActor` self _returnvalue)
  (set `ProjectileBase.OwningController` (`self.GetController`) _returnvalue)
  (`ProjectileBase.ClearIgnoredActors` _returnvalue)
  (`ProjectileBase.AddIgnoredActor` _returnvalue self))

(fn `UserConstructionScript`)