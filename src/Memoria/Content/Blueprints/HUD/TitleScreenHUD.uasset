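; Title screen HUD actor that shows the title menu and hands off to the first map selection screen.
; On BeginPlay it creates the WBP_TitleScreen widget, adds it to the viewport and binds to its FadeoutComplete event.
; StartGame plays the title widget's FadeOutMenu animation, and the FadeoutComplete handler then creates and displays WBP_FirstMapSelection.
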(event `self.ReceiveBeginPlay`
  (bind _returnvalue (`|CreateWidget` "/Game/Widgets/WBP_TitleScreen.WBP_TitleScreen_C" (`GameplayStatics.GetPlayerController` 0)))
  (set `self.TitleScreen` _returnvalue)
  (`UserWidget.AddToViewport` _returnvalue 0)
  (add `/Game/Widgets/WBP_TitleScreen.FadeoutComplete` _returnvalue (delegate `FadeoutComplete_Event_0`)))

(event `FadeoutComplete_Event_0`
  (bind _returnvalue (`|CreateWidget` "/Game/Widgets/WBP_FirstMapSelection.WBP_FirstMapSelection_C"))
  (`UserWidget.AddToViewport` _returnvalue 0))

(fn `StartGame`
  (bind _titlescreen (`self.TitleScreen`)
    (:`then`
      (`UserWidget.PlayAnimation` _titlescreen (`/Game/Widgets/WBP_TitleScreen.FadeOutMenu` _titlescreen) 0.0 1 "Forward" 1.0))
    (:`else`)))

(fn `UserConstructionScript`)