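; Black hole projectile that pulls nearby enemies toward its Horizon component.
; Every Tick it finds BP_EnemyBase actors overlapping Sphere1 and applies a CharacterMovement impulse along the look-at direction to Horizon.
; The pull has fixed strength, unscaled by distance or delta time.
; Disconnected leftover nodes hold an unused velocity-change impulse and a capsule velocity reset.
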(event `self.ReceiveTick`
  (params (DeltaSeconds :type "Float (single-precision)"))
  (for _array_element (`PrimitiveComponent.GetOverlappingActors` (`self.Sphere1`) "/Game/Blueprints/BP_EnemyBase.BP_EnemyBase_C")
    (bind _asbp_enemy_base (cast `/Game/Blueprints/BP_EnemyBase` _array_element))
    (`CharacterMovementComponent.AddImpulse` (`Character.CharacterMovement` _asbp_enemy_base) (* (`KismetMathLibrary.GetForwardVector` (`KismetMathLibrary.FindLookAtRotation` (`SceneComponent.K2_GetComponentLocation` (`Actor.RootComponent` _asbp_enemy_base)) (`SceneComponent.K2_GetComponentLocation` (`self.Horizon`)))) 50000.0) false)))

(event `self.ReceiveActorBeginOverlap`
  (params (OtherActor :type "Actor Object Reference")))

(fn `UserConstructionScript`)