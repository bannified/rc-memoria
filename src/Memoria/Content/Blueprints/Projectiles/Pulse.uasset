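; Pulse is a projectile Blueprint that drags enemies toward the centre of its AOE component.
; Each tick it moves every overlapping BP_EnemyBase by the full horizontal offset to that centre, using a swept world transform so collisions can stop the move.
; If a sweep is blocked by an actor not friendly to the moved enemy, the Pulse destroys itself.
; BeginPlay, overlap and construction only call the parent.
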(event `self.ReceiveBeginPlay`
  (`parent.ReceiveBeginPlay`))

(event `self.ReceiveActorBeginOverlap`
  (params (OtherActor :type "Actor Object Reference"))
  (`parent.ReceiveActorBeginOverlap` OtherActor))

(event `self.ReceiveTick`
  (params (DeltaSeconds :type "Float (single-precision)"))
  (bind _aoe (`self.AOE`))
  (`parent.ReceiveTick` DeltaSeconds)
  (for _array_element (`PrimitiveComponent.GetOverlappingActors` _aoe "/Game/Blueprints/BP_EnemyBase.BP_EnemyBase_C")
    (bind _sweephitresult (`SceneComponent.K2_AddWorldTransform` (`Actor.RootComponent` _array_element) (`KismetMathLibrary.Conv_VectorToTransform` (`KismetMathLibrary.MakeVector` (.x (- (`SceneComponent.K2_GetComponentLocation` _aoe) (`SceneComponent.K2_GetComponentLocation` (`Actor.RootComponent` _array_element)))) (.y (- (`SceneComponent.K2_GetComponentLocation` _aoe) (`SceneComponent.K2_GetComponentLocation` (`Actor.RootComponent` _array_element)))) 0.0)) true false))
    (bind (_bblockinghit _binitialoverlap _time _distance _location _impactpoint _normal _impactnormal _physmat _hitactor) (`GameplayStatics.BreakHitResult` _sweephitresult))
    (bind _returnvalue (`HealthComponent.IsFriendly` _hitactor _array_element))
    (if _returnvalue
      _
      (elif _bblockinghit
        (`self.K2_DestroyActor`)))))

(fn `UserConstructionScript`
  (`parent.UserConstructionScript`))