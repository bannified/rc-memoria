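; Base game mode for Memoria that runs the level intro and the between-level flow.
; BeginPlay disables input and plays the game-start widget; StartGameImmediate re-enables input and starts the current level's data asset.
; Closing the perk screen opens the loadout screen, whose close saves and alternates between Map1Deco and Map0Deco.
; Perks and attacks persist through the game instance; TryLoadGame restores them, except the saved special attacks.
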(event `self.ReceiveBeginPlay`
  (`self.PlayGameIntro`)
  (bind _asbp_player_character_base (cast `/Game/Blueprints/BP_PlayerCharacterBase` (`GameplayStatics.GetPlayerPawn` 0)))
  (add `/Game/Blueprints/BP_PlayerCharacterBase.OnPerkScreenClose` _asbp_player_character_base (delegate `OnPerkScreenClose`)))

(event `OnPerkScreenClose`
  (`/Game/Blueprints/BP_PlayerCharacterBase.OpenLoadoutScreen` (stale `self.ReceiveBeginPlay` _asbp_player_character_base)))

(event `OnLoadoutScreenClosed`
  (`self.SaveGame`)
  (`self.StartNextLevel`))

(fn `PlayGameIntro`
  (bind _returnvalue (`GameplayStatics.GetPlayerController` 0))
  (`self.DisableInput` _returnvalue _returnvalue)
  (bind _returnvalue_2 (`|CreateWidget` "/Game/Widgets/GameModes/WBP_GameStart.WBP_GameStart_C" _returnvalue))
  (add `/Game/Widgets/GameModes/WBP_GameStart.WBP_GameStartAnimationDone` _returnvalue_2 (`|CreateDelegate` :!event `StartGameImmediate`))
  (`UserWidget.AddToPlayerScreen` _returnvalue_2 200)
  (`/Game/Widgets/GameModes/WBP_GameStart.Play` _returnvalue_2))

(fn `SaveGame`
  (bind _asbp_player_character_base (cast `/Game/Blueprints/BP_PlayerCharacterBase` (`GameplayStatics.GetPlayerPawn` 0)))
  (bind _asbp_memoria_game_instance (cast `/Game/GameplayData/BP_MemoriaGameInstance` (`GameplayStatics.GetGameInstance`)))
  (bind _output_get (set `/Game/Blueprints/BP_PlayerCharacterBase.GameInstance` _asbp_memoria_game_instance _asbp_player_character_base))
  (set `/Game/GameplayData/BP_MemoriaGameInstance.PlayerPerkMap` (`/Game/Blueprints/BP_PlayerCharacterBase.PerkMap` _asbp_player_character_base) _output_get)
  (set `/Game/GameplayData/BP_MemoriaGameInstance.CharAttackClasses` (`CharacterBase.AttacksClasses` _asbp_player_character_base) _output_get)
  (set `/Game/GameplayData/BP_MemoriaGameInstance.SpecialAttack1` (`/Game/Blueprints/BP_PlayerCharacterBase.SpecialAttack1` _asbp_player_character_base) _output_get)
  (set `/Game/GameplayData/BP_MemoriaGameInstance.SpecialAttack2` (`/Game/Blueprints/BP_PlayerCharacterBase.SpecialAttack2` _asbp_player_character_base) _output_get)
  (set `/Game/GameplayData/BP_MemoriaGameInstance.HasSave` true _output_get))

(fn `StartGameImmediate`
  (bind _returnvalue (`GameplayStatics.GetPlayerController` 0))
  (`self.EnableInput` _returnvalue _returnvalue)
  (`self.StartGame` (`self.CurrentLevelDataAsset`)))

(fn `StartNextLevel`
  (bind _returnvalue (`GameplayStatics.GetCurrentLevelName` true))
  (if (`KismetStringLibrary.EqualEqual_StrStr` _returnvalue "Map1Deco")
    (`GameplayStatics.OpenLevel` "Map0Deco")
    (else
      (`GameplayStatics.OpenLevel` "Map1Deco"))))

(fn `TryLoadGame`
  (bind _asbp_player_character_base (cast `/Game/Blueprints/BP_PlayerCharacterBase` (`GameplayStatics.GetPlayerPawn` 0)))
  (bind _asbp_memoria_game_instance (cast `/Game/GameplayData/BP_MemoriaGameInstance` (`GameplayStatics.GetGameInstance`)))
  (bind _output_get (set `/Game/Blueprints/BP_PlayerCharacterBase.GameInstance` _asbp_memoria_game_instance _asbp_player_character_base))
  (if (`/Game/GameplayData/BP_MemoriaGameInstance.HasSave` _output_get)
    (set `/Game/Blueprints/BP_PlayerCharacterBase.PerkMap` (`/Game/GameplayData/BP_MemoriaGameInstance.PlayerPerkMap` _asbp_memoria_game_instance) _asbp_player_character_base)
    (set `CharacterBase.AttacksClasses` (`/Game/GameplayData/BP_MemoriaGameInstance.CharAttackClasses` _asbp_memoria_game_instance) _asbp_player_character_base)
    (`/Game/Blueprints/BP_PlayerCharacterBase.InitPerks` _asbp_player_character_base)
    (`/Game/Blueprints/BP_PlayerCharacterBase.InitAttacks` _asbp_player_character_base)))

(fn `UserConstructionScript`)