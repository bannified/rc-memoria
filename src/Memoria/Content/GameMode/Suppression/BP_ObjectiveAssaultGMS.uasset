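; BP_ObjectiveAssaultGMS is the Suppression game mode state for the Objective Assault phase, handling that phase's player-facing UI.
; On enter, it requires a BP_SuppressionGameController, plays a transition intro widget on screen and adds an objective assault info box to the player character's HUD.
; On exit, it removes the stored box from that HUD, working only with player controller 0.
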(event `self.ReceiveOnStateEnter`
  (params (GameMode :type "GameControllerBase Object Reference"))
  (bind _returnvalue (`GameplayStatics.GetPlayerController` 0))
  (cast `/Game/GameMode/Suppression/BP_SuppressionGameController` GameMode)
  ;[1 1 1] Intro
  (bind _returnvalue_2 (`|CreateWidget` "/Game/Widgets/GameModes/Suppression/WBP_ToObjectiveAssault.WBP_ToObjectiveAssault_C" _returnvalue))
  (`/Game/Widgets/GameModes/Suppression/WBP_ToObjectiveAssault.Play` _returnvalue_2)
  (`UserWidget.AddToPlayerScreen` _returnvalue_2 500)
  (bind _asbp_player_character_base (cast `/Game/Blueprints/BP_PlayerCharacterBase` (`Controller.K2_GetPawn` _returnvalue)))
  (bind _playerhudwidget (`/Game/Blueprints/BP_PlayerCharacterBase.PlayerHUDWidget` _asbp_player_character_base)
    (:`then`
      (bind _returnvalue_3 (`|CreateWidget` "/Game/Widgets/GeneralGameplayWidgets/GameplayInfoWidgets/WBP_Suppression_ObjectiveAssault_Box.WBP_Suppression_ObjectiveAssault_Box_C"))
      (set `self.ObjectiveAssaultBox` _returnvalue_3)
      (`/Game/Widgets/GeneralGameplayWidgets/WBP_PlayerHUD.AddGameplayInfoWidget` _playerhudwidget _returnvalue_3))
    (:`else`)))

(event `self.ReceiveOnStateExit`
  (params (GameMode :type "GameControllerBase Object Reference"))
  (bind _asbp_player_character_base (cast `/Game/Blueprints/BP_PlayerCharacterBase` (`Controller.K2_GetPawn` (`GameplayStatics.GetPlayerController` 0))))
  (bind _playerhudwidget (`/Game/Blueprints/BP_PlayerCharacterBase.PlayerHUDWidget` _asbp_player_character_base)
    (:`then`
      (bind _objectiveassaultbox (`self.ObjectiveAssaultBox`)
        (:`then`
          (`/Game/Widgets/GeneralGameplayWidgets/WBP_PlayerHUD.RemoveGameplayInfoWidget` _playerhudwidget _objectiveassaultbox))
        (:`else`)))
    (:`else`)))

(fn `UserConstructionScript`)