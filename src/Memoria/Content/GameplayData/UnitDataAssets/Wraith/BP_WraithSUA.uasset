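; Unit data asset for the Wraith miniboss that applies its tuning values to the boss's attacks when the unit initializes.
; InitializeUnit calls the parent, then casts the first three attack slots to burst fire, rocket and homing attack types.
; Each gets its projectile class and modifiable-attribute base values for burst, spread or timing.
; A failed cast silently skips every step after it.
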(event `self.InitializeUnit`
  (params (Actor :type "Actor Object Reference"))
  (`parent.InitializeUnit` Actor)
  (bind _asbp_wraith_miniboss (cast `/Game/Blueprints/Enemies/Wraith_Miniboss/BP_Wraith_Miniboss` Actor))
  (bind _attacks (`CharacterBase.Attacks` _asbp_wraith_miniboss))
  (bind _asbp_burst_projectile_fire (cast `/Game/Blueprints/Characters/BP_BurstProjectileFire` (`|GetArrayItem` _attacks)))
  (set `ProjectileAttack.ProjectileClass` (`self.BurstProjectile`) _asbp_burst_projectile_fire)
  (`MemoriaStaticLibrary.SetModifiableAttributeBaseValue` (`BurstFireProjectileAttack.BurstCount` _asbp_burst_projectile_fire) (`KismetMathLibrary.Conv_IntToDouble` (`self.BurstCount`)))
  (`MemoriaStaticLibrary.SetModifiableAttributeBaseValue` (`BurstFireProjectileAttack.BurstInterval` _asbp_burst_projectile_fire) (`self.BurstInterval`))
  (`MemoriaStaticLibrary.SetModifiableAttributeBaseValue` (`ProjectileAttack.BulletSpreadAngle` _asbp_burst_projectile_fire) (`self.BulletSpreadAngle`))
  (bind _asbp_wraith_rocket (cast `/Game/Blueprints/Enemies/Wraith_Miniboss/BP_Wraith_Rocket` (`|GetArrayItem` _attacks 1)))
  (set `ProjectileAttack.ProjectileClass` (`self.RocketProjectile`) _asbp_wraith_rocket)
  (`MemoriaStaticLibrary.SetModifiableAttributeBaseValue` (`ProjectileAttack.BulletSpreadAngle` _asbp_wraith_rocket) (`self.RocketBulletSpreadAngle`))
  (`MemoriaStaticLibrary.SetModifiableAttributeBaseValue` (`CharacterAttack.Cooldown` _asbp_wraith_rocket) (`self.RocketCooldown`))
  (`MemoriaStaticLibrary.SetModifiableAttributeBaseValue` (`CharacterAttack.AttackDuration` _asbp_wraith_rocket) (`self.RocketAttackDuration`))
  (bind _asbp_wraith_homing_attack (cast `/Game/Blueprints/Enemies/Wraith_Miniboss/BP_WraithHomingAttack` (`|GetArrayItem` _attacks 2)))
  (set `ProjectileAttack.ProjectileClass` (`self.WraithHomingProjectile`) _asbp_wraith_homing_attack)
  (`MemoriaStaticLibrary.SetModifiableAttributeBaseValue` (`BurstFireProjectileAttack.BurstCount` _asbp_wraith_homing_attack) (`self.WraithHomingBurstCount`))
  (`MemoriaStaticLibrary.SetModifiableAttributeBaseValue` (`BurstFireProjectileAttack.BurstInterval` _asbp_wraith_homing_attack) (`self.WraithHomingBurstInterval`)))