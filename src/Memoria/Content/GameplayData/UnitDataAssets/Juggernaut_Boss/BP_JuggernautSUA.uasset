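; Unit data asset for the Juggernaut boss that applies its attack tuning values when the unit is initialized.
; After the parent initialization, it casts the actor to BP_Juggernaut and configures its Attacks array by fixed index: tracking firestorm, leaping attack, then radial firestorm.
; It copies flame area, leap and radial projectile settings onto those attacks, and any failed cast skips the remaining setup.
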(event `self.InitializeUnit`
  (params (Actor :type "Actor Object Reference"))
  (`parent.InitializeUnit` Actor)
  (bind _asbp_juggernaut (cast `/Game/Blueprints/Enemies/Juggernaut_Miniboss/BP_Juggernaut` Actor))
  (bind _attacks (`CharacterBase.Attacks` _asbp_juggernaut))
  (bind _asbp_tracking_firestorm (cast `/Game/Blueprints/Enemies/Juggernaut_Miniboss/BP_TrackingFirestorm` (`|GetArrayItem` _attacks)))
  (set `/Game/Blueprints/Enemies/Juggernaut_Miniboss/BP_TrackingFirestorm.FlameAreaScale` (`self.FlameAreaScale`) _asbp_tracking_firestorm)
  (set `/Game/Blueprints/Enemies/Juggernaut_Miniboss/BP_TrackingFirestorm.FlameAreaLifespan` (`self.FlameAreaLifespan`) _asbp_tracking_firestorm)
  (set `/Game/Blueprints/Enemies/Juggernaut_Miniboss/BP_TrackingFirestorm.FlameAreaDamagePerInterval` (`self.FlameAreaDamagePerInterval`) _asbp_tracking_firestorm)
  (bind _asbp_leaping_attack_juggernaut (cast `/Game/Blueprints/Enemies/Juggernaut_Miniboss/BP_LeapingAttack_Juggernaut` (`|GetArrayItem` _attacks 1)))
  (set `/Game/Blueprints/Enemies/Juggernaut_Miniboss/BP_LeapingAttack_Juggernaut.Radius` (`self.LeapAttackRadius`) _asbp_leaping_attack_juggernaut)
  (set `/Game/Blueprints/Enemies/Juggernaut_Miniboss/BP_LeapingAttack_Juggernaut.MaxLeapSpeed` (`self.MaxLeapSpeed`) _asbp_leaping_attack_juggernaut)
  (set `/Game/Blueprints/Enemies/Juggernaut_Miniboss/BP_LeapingAttack_Juggernaut.KnockbackStrength` (`self.KnockbackStrength`) _asbp_leaping_attack_juggernaut)
  (set `/Game/Blueprints/Enemies/Juggernaut_Miniboss/BP_LeapingAttack_Juggernaut.Damage` (`self.LeapDamage`) _asbp_leaping_attack_juggernaut)
  ;[1 1 1] Firestorm uses the player's stats for Damage
  (bind _asbp_radial_firestorm_attack (cast `/Game/Blueprints/Enemies/Juggernaut_Miniboss/BP_RadialFirestormAttack` (`|GetArrayItem` _attacks 2)))
  (set `/Game/Blueprints/Enemies/Juggernaut_Miniboss/BP_RadialFirestormAttack.NumberOfProjectiles` (`self.NumberOfRadialProjectiles`) _asbp_radial_firestorm_attack)
  (set `/Game/Blueprints/Enemies/Juggernaut_Miniboss/BP_RadialFirestormAttack.Radius` (`self.InnerRadius`) _asbp_radial_firestorm_attack))