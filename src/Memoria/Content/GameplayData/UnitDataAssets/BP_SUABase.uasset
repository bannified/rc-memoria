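; BP_SUABase is a unit data asset base that initializes a BP_CharacterBase with its stats and perks.
; InitializeUnit writes combat, movement and health values as modifiable attribute base values, then updates movement and fully restores health and mana.
; It then adds and sets up each AdditionalPerks class on the character.
; AttackDamage targets StatBaseAttackSpeed, so the later AttackSpeed write targets the same attribute.
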(event `self.InitializeUnit`
  (params (Actor :type "Actor Object Reference"))
  (bind _asbp_character_base (cast `/Game/Blueprints/BP_CharacterBase` Actor))
  (`MemoriaStaticLibrary.SetModifiableAttributeBaseValue` (`CharacterBase.StatBaseAttackSpeed` _asbp_character_base) (`self.AttackDamage`))
  (`MemoriaStaticLibrary.SetModifiableAttributeBaseValue` (`CharacterBase.StatDamageMultiplier` _asbp_character_base) (`self.AttackDamageMultiplier`))
  (`MemoriaStaticLibrary.SetModifiableAttributeBaseValue` (`CharacterBase.StatBaseAttackSpeed` _asbp_character_base) (`self.AttackSpeed`))
  (`MemoriaStaticLibrary.SetModifiableAttributeBaseValue` (`CharacterBase.StatCooldownReduction` _asbp_character_base) (`self.CooldownReduction`))
  (`MemoriaStaticLibrary.SetModifiableAttributeBaseValue` (`CharacterBase.StatAbilityDamage` _asbp_character_base) (`self.AbilityDamage`))
  (`MemoriaStaticLibrary.SetModifiableAttributeBaseValue` (`CharacterBase.StatBaseKnockback` _asbp_character_base) (`self.Knockback`))
  (`MemoriaStaticLibrary.SetModifiableAttributeBaseValue` (`CharacterBase.StatMovementSpeed` _asbp_character_base) (`self.MovementSpeed`))
  (`MemoriaStaticLibrary.SetModifiableAttributeBaseValue` (`CharacterBase.StatJumpVelocity` _asbp_character_base) (`self.JumpVelocity`))
  (`MemoriaStaticLibrary.SetModifiableAttributeBaseValue` (`CharacterBase.StatGravityScale` _asbp_character_base) (`self.GravityScale`))
  (bind _healthcomponent (`CharacterBase.HealthComponent` _asbp_character_base))
  (`MemoriaStaticLibrary.SetModifiableAttributeBaseValue` (`HealthComponent.maxHealth` _healthcomponent) (`self.MaxHealth`))
  (`MemoriaStaticLibrary.SetModifiableAttributeBaseValue` (`HealthComponent.MaxShields` _healthcomponent) (`self.MaxShields`))
  (`CharacterBase.UpdateMovementProperties` _asbp_character_base)
  (`CharacterBase.UpdateMovementProperties` _asbp_character_base)
  (`HealthComponent.FullRestoreHealthComponent` (`CharacterBase.HealthComponent` _asbp_character_base))
  (`ManaComponent.FullRestoreMana` (`CharacterBase.ManaComponent` _asbp_character_base))
  (for _array_element (`self.AdditionalPerks`)
    (bind _returnvalue (`MemoriaStaticLibrary.AddPerkToCharacterBase` _array_element _asbp_character_base))
    (`CharacterPerkComponent.Setup` _returnvalue _asbp_character_base)))